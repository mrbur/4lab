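; BP_Target is a shooting target that flips when struck by a BP_Projectile and resets after a cooldown.
; A component hit while ready clears IsReady and plays the TargetClose timeline, which drives the mesh's relative pitch.
; If the player pawn casts to BP_Turel, it waits CoolDownTime, then TargetOpen rotates the mesh again and restores IsReady on finish.
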(event OnComponentHit(SM_Target)
  (params (HitComponent :type Primitive%20Component%20Object%20Reference) (OtherActor :type Actor%20Object%20Reference) (OtherComp :type Primitive%20Component%20Object%20Reference) (NormalImpulse :type Vector :default "0, 0, 0") (Hit :type Hit%20Result%20Structure%20%28by%20ref%29))
  (if (and (== (Utilities|GetClass OtherActor) "/Game/Blueprints/BP_Projectile.BP_Projectile_C") (Variables|Default|GetisReady))
    (CallFunction|TargetHit)))

(event Custom|TargetHit
  (Variables|Default|SetisReady false)
  (bind _alpha (Timeline|TargetClose PlayFromStart)
    (:Update
      (Transformation|SetRelativeRotation (Variables|Default|GetSM_Target) (Math|Rotator|MakeRotator 0.0 (* 90 _alpha) 0.0) false false))
    (:Finished
      (Utilities|Casting|CastToBP_Turel (Game|Player|GetPlayerPawn 0))
      (Utilities|FlowControl|Delay (Variables|Default|GetCoolDownTime))
      (bind _alpha_2 (Timeline|TargetOpen PlayFromStart)
        (:Update
          (Transformation|SetRelativeRotation (Variables|Default|GetSM_Target) (Math|Rotator|MakeRotator 0.0 (* 90 _alpha_2) 0.0) false false))
        (:Finished
          (Variables|Default|SetisReady true))))))

(event EventBeginPlay)

(event Collision|EventActorBeginOverlap
  (params (OtherActor :type Actor%20Object%20Reference)))

(event EventTick
  (params (DeltaSeconds :type Float%20%28single-precision%29)))

(fn ConstructionScript)