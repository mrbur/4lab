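; Player-controlled turret that fires projectiles with left mouse and twin laser beams while right mouse is held.
; Movement axes drive clamped pitch and free yaw, passed to ABP_Turel for aiming.
; The laser toggles two Niagara beams and an anim flag, running debug-drawn pawn traces from both every tick.
; Both traces print the hit actor, but only the second calls Dam on BP_DummyAI.
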(event Custom|TurelHit
  (Development|PrintString "Hello"))

(event EventBeginPlay
  (bind _asabp_turel (Utilities|Casting|CastToABP_Turel (Components|SkeletalMesh|GetAnimInstance (Variables|Default|GetSK_Turel))))
  (Variables|Default|SetABPInstance _asabp_turel)
  (Components|Activation|Deactivate (Variables|Default|GetNiagara))
  (Components|Activation|Deactivate (Variables|Default|GetNiagara1)))

(event Collision|EventActorBeginOverlap
  (params (OtherActor :type Actor%20Object%20Reference)))

(event EventTick
  (params (DeltaSeconds :type Float%20%28single-precision%29))
  (if (Variables|Default|GetIsLaser)
    (CallFunction|Trace)
    (CallFunction|Trace2)))

(event Input|AxisEvents|InputAxisMoveRight
  (params (AxisValue :type Float%20%28single-precision%29))
  (bind _output_get (Variables|Default|SetCurrentHRotation (+ (* AxisValue (Utilities|Time|GetWorldDeltaSeconds) (Variables|Default|GetHRotationSpeed)) (Variables|Default|GetCurrentHRotation))))
  (Variables|/Game/SkeletalMesh/ABP_Turel.ABP_Turel_C|SetHrotation (Variables|Default|GetABPInstance) _output_get))

(event Input|AxisEvents|InputAxisMoveForward
  (params (AxisValue :type Float%20%28single-precision%29))
  (bind _output_get (Variables|Default|SetCurrentVRotation (Math|Float|Clamp(Float) (+ (* AxisValue (Utilities|Time|GetWorldDeltaSeconds) (Variables|Default|GetVRotationSpeed) -1.0) (Variables|Default|GetCurrentVRotation)) -6e+01 1e+01)))
  (Variables|/Game/SkeletalMesh/ABP_Turel.ABP_Turel_C|SetVRotation (Variables|Default|GetABPInstance) _output_get))

(event Input|MouseEvents|LeftMouseButton
  (params (Key :type Key%20Structure))
  (bind _projectilespawnlocation (Variables|Default|GetProjectileSpawnLocation))
  (bind _returnvalue (Transformation|GetWorldTransform _projectilespawnlocation))
  (:Pressed
    (Game|SpawnActorfromClass "/Game/Blueprints/BP_Projectile.BP_Projectile_C" (Math|Transform|MakeTransform (.location _returnvalue) (.rotation _returnvalue) "1,1,1") "Undefined" 0 0)))

(event Input|MouseEvents|RightMouseButton
  (params (Key :type Key%20Structure))
  (bind _niagara (Variables|Default|GetNiagara))
  (bind _niagara1 (Variables|Default|GetNiagara1))
  (:Pressed
    (Variables|Default|SetIsLaser true)
    (Variables|/Game/SkeletalMesh/ABP_Turel.ABP_Turel_C|SetLaserCharged (Variables|Default|GetABPInstance) true)
    (Components|Activation|Activate _niagara true)
    (Components|Activation|Activate _niagara1 true)
    (CallFunction|Trace))
  (:Released
    (Variables|Default|SetIsLaser false)
    (Variables|/Game/SkeletalMesh/ABP_Turel.ABP_Turel_C|SetLaserCharged (Variables|Default|GetABPInstance) false)
    (Components|Activation|Deactivate _niagara)
    (Components|Activation|Deactivate _niagara1)))

(fn ConstructionScript)

(fn Trace
  (bind _niagara (Variables|Default|GetNiagara))
  (bind _returnvalue (Transformation|GetWorldLocation _niagara))
  (bind _outhit (Collision|LineTraceForObjects _returnvalue (+ _returnvalue (* (Math|Vector|GetForwardVector (Transformation|GetWorldRotation _niagara)) 1000)) (Utilities|Array|MakeArray "ObjectTypeQuery3") false 0 "ForOneFrame"))
  (Development|PrintString (Utilities|GetDisplayName (.HitActor (Collision|BreakHitResult _outhit))))
  (return (.HitActor (Collision|BreakHitResult _outhit))))

(fn Trace2
  (bind _niagara1 (Variables|Default|GetNiagara1))
  (bind _returnvalue (Transformation|GetWorldLocation _niagara1))
  (bind _outhit (Collision|LineTraceForObjects _returnvalue (+ _returnvalue (* (Math|Vector|GetForwardVector (Transformation|GetWorldRotation _niagara1)) 1000)) (Utilities|Array|MakeArray "ObjectTypeQuery3") false 0 "ForOneFrame"))
  (Development|PrintString (Utilities|GetDisplayName (.HitActor (Collision|BreakHitResult _outhit))))
  (bind _asbp_dummy_ai (Utilities|Casting|CastToBP_DummyAI (.HitActor (Collision|BreakHitResult _outhit))))
  (Default|Dam _asbp_dummy_ai)
  (return (.HitActor (Collision|BreakHitResult _outhit))))