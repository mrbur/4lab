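; BP_DummyAI is a target character that ragdolls and stops moving when damaged.
; Capsule hits call Dam, which bumps the score on the first WI_PlayerUI found if the other actor is a BP_Projectile.
; Otherwise Dam needs a WI_PlayerUI argument to bump the laser count and ragdoll; capsule hits pass none.
; Tick's proximity check casts the player pawn to BP_Turel but does nothing further.
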(event OnComponentHit(CapsuleComponent)
  (params (HitComponent :type Primitive%20Component%20Object%20Reference) (OtherActor :type Actor%20Object%20Reference) (OtherComp :type Primitive%20Component%20Object%20Reference) (NormalImpulse :type Vector :default "0, 0, 0") (Hit :type Hit%20Result%20Structure%20%28by%20ref%29))
  (CallFunction|Dam OtherActor))

(event EventBeginPlay)

(event Collision|EventActorBeginOverlap
  (params (OtherActor :type Actor%20Object%20Reference)))

(event EventTick
  (params (DeltaSeconds :type Float%20%28single-precision%29))
  (if (Math|Vector|Equal(Vector) (Transformation|GetActorLocation) (Transformation|GetActorLocation (Game|Player|GetPlayerPawn 0)) 1.5e+02)
    (Utilities|Casting|CastToBP_Turel (Game|Player|GetPlayerPawn 0))))

(fn ConstructionScript)

(fn Dam
  (params (NewParam :type Actor%20Object%20Reference) (widget :type User%20Widget%20Object%20Reference))
  (if (== (Utilities|GetClass NewParam) "/Game/Blueprints/BP_Projectile.BP_Projectile_C")
    (bind _foundwidgets (Widget|GetAllWidgetsOfClass "/Game/Widgets/WI_PlayerUI.WI_PlayerUI_C" false))
    (bind _aswi_player_ui (Utilities|Casting|CastToWI_PlayerUI (Utilities|Array|Get(acopy) _foundwidgets)))
    (Default|ScoreInc _aswi_player_ui)
    (else
      (bind _aswi_player_ui_2 (Utilities|Casting|CastToWI_PlayerUI widget))
      (Default|LaserInc _aswi_player_ui_2)))
  (Physics|SetSimulatePhysics (Variables|Character|GetMesh) true)
  (Pawn|Components|CharacterMovement|DisableMovement (Variables|Character|GetCharacterMovement)))